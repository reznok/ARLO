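; GA_JumpGMCBool_WithCost is a hero gameplay ability that triggers a jump through the GMC movement component while paying the ability's cost.
; On activation it finds the owner's ALMovementComponent, checks CanJump for grounded or extra-jump eligibility, then commits the ability.
; Only on a successful commit does it set the GMC bound WantsToJump bool, leaving the jump itself to movement; every path ends the ability immediately.
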(event `self.K2_ActivateAbility`
  (bind _returnvalue (`Actor.GetComponentByClass` (`self.GetOwningActorFromActorInfo`) "/Script/Arlo.ALMovementComponent"))
  (`/Engine/EditorBlueprintResources/StandardMacros.IsValid` _returnvalue
    (:`Is Valid`
      (bind _output_get (set `self.GMCMovementComponent` _returnvalue))
      ;[0 0.7174 1] IsGrounded / ExtraJumps check
      (bind _returnvalue_2 (`ALMovementComponent.CanJump` _output_get))
      (if _returnvalue_2
        (bind _returnvalue_3 (`self.K2_CommitAbility`))
        (if _returnvalue_3
          ;[0 0.7174 1] Set GMC Bound Bool
          (set `ALMovementComponent.bWantsToJump` true (`self.GMCMovementComponent`))
          (`self.K2_EndAbility`)
          (else
            (`self.K2_EndAbility` :!label _label)))
        (else
          (goto _label))))
    (:`Is Not Valid`
      (goto _label))))